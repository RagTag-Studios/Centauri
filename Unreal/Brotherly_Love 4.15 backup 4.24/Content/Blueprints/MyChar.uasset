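; Player character Blueprint that handles movement, look, sprinting and a flashlight.
; Move and look axis inputs follow the control rotation and are gated by a BlockInput flag.
; Holding Left Shift raises the walk speed until release, independent of that flag.
; The Flashlight action toggles SpotLight visibility, and mouse X/Y events align the light to the control rotation.
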(event `InputAxis|MoveForward`
  (params (AxisValue :type "Float (single-precision)"))
  ;[1 1 1] Player_Movement
  (if (not (`self.BlockInput`))
    (`self.AddMovementInput` (`KismetMathLibrary.GetForwardVector` (`self.GetControlRotation`)) AxisValue)))

(event `InputAction|Flashlight`
  (params (Key :type "Key Structure" :default "AnyKey"))
  (bind _spotlight (`self.SpotLight`))
  ;[1 1 1] Flashlight
  (:`Pressed`
    (`/Engine/EditorBlueprintResources/StandardMacros.FlipFlop`
      (:`A`
        (`SceneComponent.ToggleVisibility` _spotlight false))
      (:`B`
        (`SceneComponent.ToggleVisibility` _spotlight false)))))

(event `InputAxisKey|MouseX`
  (params (AxisValue :type "Float (single-precision)"))
  ;[1 1 1] Flashlight
  (`SceneComponent.K2_SetWorldRotation` (`self.SpotLight`) (`self.GetControlRotation`) false false :!label _label))

(event `InputAxisKey|MouseY`
  (params (AxisValue :type "Float (single-precision)"))
  ;[1 1 1] Flashlight
  (goto _label))

(event `InputAxis|MoveRight`
  (params (AxisValue :type "Float (single-precision)"))
  ;[1 1 1] Player_Movement
  (if (not (`self.BlockInput`))
    (`self.AddMovementInput` (`KismetMathLibrary.GetRightVector` (`self.GetControlRotation`)) AxisValue)))

(event `InputAxis|LookUp`
  (params (AxisValue :type "Float (single-precision)"))
  ;[1 1 1] Player_Movement
  (if (not (`self.BlockInput`))
    (`self.AddControllerPitchInput` AxisValue)))

(event `InputAxis|Turn`
  (params (AxisValue :type "Float (single-precision)"))
  ;[1 1 1] Player_Movement
  (if (not (`self.BlockInput`))
    (`self.AddControllerYawInput` AxisValue)))

(event `Key|LeftShift`
  (params (Key :type "Key Structure" :default "AnyKey"))
  (bind _charactermovement (`self.CharacterMovement`))
  ;[1 1 1] Player_Movement
  (:`Pressed`
    (set `CharacterMovementComponent.MaxWalkSpeed` 300.0 _charactermovement))
  (:`Released`
    (set `CharacterMovementComponent.MaxWalkSpeed` 150.0 _charactermovement)))

(fn `UserConstructionScript`)