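; LSwitch2 is an interactive light switch that MyChar toggles with E to signal Room 1 on or off.
; Box overlap enables and disables player input on the switch.
; A press plays the up or down Level Sequence, waits briefly, then calls BRoom1On or BRoom1Off.
; HasEBeenPressed blocks repeat presses during the delay, and the switch state is tracked in a boolean named IsDoorOpen.
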(event `self.Box.OnComponentBeginOverlap`
  (params (OverlappedComponent :type "PrimitiveComponent Object Reference") (OtherActor :type "Actor Object Reference") (OtherComp :type "PrimitiveComponent Object Reference") (OtherBodyIndex :type Integer) (bFromSweep :type Boolean) (SweepResult :type "HitResult Structure (by ref)"))
  ;[1 1 1] Switch_Light
  (cast `/Game/Blueprints/MyChar` OtherActor)
  (`KismetSystemLibrary.PrintString` "In Box")
  (`self.EnableInput` (`GameplayStatics.GetPlayerController` 0)))

(event `self.Box.OnComponentEndOverlap`
  (params (OverlappedComponent :type "PrimitiveComponent Object Reference") (OtherActor :type "Actor Object Reference") (OtherComp :type "PrimitiveComponent Object Reference") (OtherBodyIndex :type Integer))
  ;[1 1 1] Switch_Light
  (cast `/Game/Blueprints/MyChar` OtherActor)
  (`self.DisableInput` (`GameplayStatics.GetPlayerController` 0)))

(event `Key|E`
  (params (Key :type "Key Structure" :default "AnyKey"))
  ;[1 1 1] Switch_Light
  (:`Pressed`
    (if (not (`self.HasEBeenPressed`))
      (set `self.HasEBeenPressed` true)
      (if (`self.IsDoorOpen`)
        (bind _returnvalue (`LevelSequencePlayer.CreateLevelSequencePlayer` "/Game/Cinematics/Switches/LSwitch2_Down.LSwitch2_Down"))
        (`MovieSceneSequencePlayer.Play` _returnvalue)
        (else
          (bind _returnvalue_2 (`LevelSequencePlayer.CreateLevelSequencePlayer` "/Game/Cinematics/Switches/LSwitch2_Up.LSwitch2_Up"))
          (`MovieSceneSequencePlayer.Play` _returnvalue_2)))
      (`KismetSystemLibrary.Delay` 0.5)
      (if (`self.IsDoorOpen`)
        (`self.BRoom1_Off`)
        (else
          (`self.BRoom1_On`)))
      (set `self.HasEBeenPressed` false)
      (if (`self.IsDoorOpen`)
        (set `self.IsDoorOpen` false)
        (else
          (set `self.IsDoorOpen` true))))))

(fn `UserConstructionScript`
  (`parent.UserConstructionScript`))