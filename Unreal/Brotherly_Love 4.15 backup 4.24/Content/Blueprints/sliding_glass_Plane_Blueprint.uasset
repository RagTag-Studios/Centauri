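; Sliding glass door Blueprint that MyChar opens or closes with E while inside its trigger box.
; Box overlaps enable and disable input, and each press plays an open or close Level Sequence with sound, using delays and a flag to block repeat presses.
; Opening starts the outside ambience, and closing stops it unless AmbianceSwitch is set by the AmbianceON and AmbianceOFF triggers.
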(event `self.Box.OnComponentBeginOverlap`
  (params (OverlappedComponent :type "PrimitiveComponent Object Reference") (OtherActor :type "Actor Object Reference") (OtherComp :type "PrimitiveComponent Object Reference") (OtherBodyIndex :type Integer) (bFromSweep :type Boolean) (SweepResult :type "HitResult Structure (by ref)"))
  ;[1 1 1] Input
  (cast `/Game/Blueprints/MyChar` OtherActor)
  (`KismetSystemLibrary.PrintString` "In Box")
  (`self.EnableInput` (`GameplayStatics.GetPlayerController` 0)))

(event `self.Box.OnComponentEndOverlap`
  (params (OverlappedComponent :type "PrimitiveComponent Object Reference") (OtherActor :type "Actor Object Reference") (OtherComp :type "PrimitiveComponent Object Reference") (OtherBodyIndex :type Integer))
  ;[1 1 1] Input
  (cast `/Game/Blueprints/MyChar` OtherActor)
  (`self.DisableInput` (`GameplayStatics.GetPlayerController` 0)))

(event `Key|E`
  (params (Key :type "Key Structure" :default "AnyKey"))
  (bind _ambient_outside (`self.Ambient_Outside`))
  ;[1 1 1] Cinematic
  (:`Pressed`
    (if (not (`self.HasEBeenPressed`))
      (set `self.HasEBeenPressed` true)
      (if (`self.IsDoorOpen`)
        (bind _returnvalue (`LevelSequencePlayer.CreateLevelSequencePlayer` "/Game/Cinematics/Door_Sequences/Sliding_Glass_Close.Sliding_Glass_Close"))
        (`MovieSceneSequencePlayer.Play` _returnvalue)
        (`KismetSystemLibrary.Delay` 0.4)
        (`AudioComponent.Play` (`self.SlidingClose`) 0.0)
        (`KismetSystemLibrary.Delay` 2.15)
        (if (not (`self.AmbianceSwitch`))
          (`AudioComponent.Stop` _ambient_outside))
        (else
          (bind _returnvalue_2 (`LevelSequencePlayer.CreateLevelSequencePlayer` "/Game/Cinematics/Door_Sequences/Sliding_Glass_Open.Sliding_Glass_Open"))
          (`MovieSceneSequencePlayer.Play` _returnvalue_2)
          (`AudioComponent.Play` (`self.SlidingOpen`) 0.0)
          (`KismetSystemLibrary.Delay` 0.35)
          (`AudioComponent.Play` _ambient_outside 0.0)
          (`KismetSystemLibrary.Delay` 2.15)))
      (set `self.HasEBeenPressed` false)
      (if (`self.IsDoorOpen`)
        (set `self.IsDoorOpen` false)
        (else
          (set `self.IsDoorOpen` true))))))

(event `self.AmbianceON.OnComponentBeginOverlap`
  (params (OverlappedComponent :type "PrimitiveComponent Object Reference") (OtherActor :type "Actor Object Reference") (OtherComp :type "PrimitiveComponent Object Reference") (OtherBodyIndex :type Integer) (bFromSweep :type Boolean) (SweepResult :type "HitResult Structure (by ref)"))
  ;[1 1 1] Ambiance_Switch
  (cast `/Game/Blueprints/MyChar` OtherActor)
  (set `self.AmbianceSwitch` true))

(event `self.AmbianceOFF.OnComponentBeginOverlap`
  (params (OverlappedComponent :type "PrimitiveComponent Object Reference") (OtherActor :type "Actor Object Reference") (OtherComp :type "PrimitiveComponent Object Reference") (OtherBodyIndex :type Integer) (bFromSweep :type Boolean) (SweepResult :type "HitResult Structure (by ref)"))
  ;[1 1 1] Ambiance_Switch
  (cast `/Game/Blueprints/MyChar` OtherActor)
  (set `self.AmbianceSwitch` false))

(fn `UserConstructionScript`)